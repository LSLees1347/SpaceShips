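; BP_ShipBase is a player-controlled ship that separates free camera look from the direction of travel.
; Enhanced Input drives thrust along the actor's forward vector through ShipMovement, while look input feeds controller yaw and pitch.
; Pressing Select captures the camera's forward direction, then the MakeNewRotation timeline lerps the ship's rotation to it along the shortest path.
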(event `EnhancedInput|/Game/Input/IA_Thrust`
  (params (ActionValue :type Boolean) (ElapsedSeconds :type "Float (double-precision)") (TriggeredSeconds :type "Float (double-precision)") (InputAction :type "InputAction Object Reference" :default "/Game/Input/IA_Thrust.IA_Thrust"))
  (:`Triggered`
    (`PawnMovementComponent.AddInputVector` (`self.ShipMovement`) (`self.GetActorForwardVector`) false)))

(event `EnhancedInput|/Game/Input/IA_Look`
  (params (ActionValue :type "Vector2D Structure") (ElapsedSeconds :type "Float (double-precision)") (TriggeredSeconds :type "Float (double-precision)") (InputAction :type "InputAction Object Reference" :default "/Game/Input/IA_Look.IA_Look"))
  (:`Triggered`
    (`self.AddControllerYawInput` ActionValue_X)
    (`self.AddControllerPitchInput` ActionValue_Y)))

(event `EnhancedInput|/Game/Input/IA_Select`
  (params (ActionValue :type Boolean) (ElapsedSeconds :type "Float (double-precision)") (TriggeredSeconds :type "Float (double-precision)") (InputAction :type "InputAction Object Reference" :default "/Game/Input/IA_Select.IA_Select"))
  (bind _returnvalue (`SceneComponent.K2_GetComponentLocation` (`self.StaticMesh`)))
  (:`Started`
    (set `self.OldRotation` (`self.K2_GetActorRotation`))
    (set `self.NewRotation` (`KismetMathLibrary.FindLookAtRotation` _returnvalue (+ _returnvalue (`SceneComponent.GetForwardVector` (`self.Camera`)))))
    (bind (_direction _turn) (`Timeline|MakeNewRotation` :!via `PlayFromStart`)
      (:`Update`
        (`self.K2_SetActorRotation` (`KismetMathLibrary.RLerp` (`self.OldRotation`) (`self.NewRotation`) _turn true))))))

(fn `UserConstructionScript`)